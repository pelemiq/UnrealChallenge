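; BP_MapNode is a map node actor that holds a list of connections to other actors.
; Hovering the cursor over it swaps the Cylinder mesh to a hover material, and moving off restores the default.
; A DebugDrawConnections event draws temporary debug arrows from the node to each connected actor.
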(event Custom|DebugDrawConnections
  (for _array_element (Variables|Default|GetConnections)
    (Rendering|Debug|DrawDebugArrow (Transformation|GetActorLocation) (Transformation|GetActorLocation _array_element) 1e+01 "(R=0.772894,G=0.390584,B=0.979167,A=1.000000)" 5.0 2.0)))

(event EventBeginPlay)

(event Collision|EventActorBeginOverlap
  (params (OtherActor :type Actor%20Object%20Reference)))

(event EventTick
  (params (DeltaSeconds :type Float%20%28single-precision%29)))

(event MouseInput|EventActorBeginCursorOver
  (Rendering|Material|SetMaterial (Variables|Default|GetCylinder) 0 "/Game/Challenges/Challenge1/Materials/M_MapNode_Hover.M_MapNode_Hover"))

(event MouseInput|EventActorEndCursorOver
  (Rendering|Material|SetMaterial (Variables|Default|GetCylinder) 0 "/Game/Challenges/Challenge1/Materials/M_MapNode.M_MapNode"))

(fn ConstructionScript)